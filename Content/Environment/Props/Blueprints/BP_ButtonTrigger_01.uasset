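; A button prop that a laser switches on to open a door for a limited time.
; When a laser overlaps it, the button kills the laser, turns its dynamic material green and opens the door.
; After a configurable delay it always reverts to red and closes the door.
; The construction script creates the material and loops over all BP_Door actors, keeping only the last one as its target.
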(event `self.ReceiveActorBeginOverlap`
  (params (OtherActor :type "Actor Object Reference")))

(event `self.LaserTick`
  (params (Laser :type "LaserBase Object Reference") (DeltaSeconds :type "Float (single-precision)")))

(event `self.LaserBeginOverlap`
  (params (Laser :type "LaserBase Object Reference"))
  (`LaserBase.Kill` Laser true)
  (set `self.IsOn` true)
  (`MaterialInstanceDynamic.SetVectorParameterValue` (`self.DynaMat`) "ButtonColor" (struct :`G` 1.0 :`A` 1.0))
  (bind _asbp_door (cast `/Game/Environment/Props/Blueprints/BP_Door` (`self.Door`)))
  (`/Game/Environment/Props/Blueprints/BP_Door.Open` _asbp_door)
  (if true
    (`KismetSystemLibrary.Delay` (`self.Delay`))
    (set `self.IsOn` false)
    (`MaterialInstanceDynamic.SetVectorParameterValue` (`self.DynaMat`) "ButtonColor" (struct :`R` 1.0 :`A` 1.0))
    (bind _asbp_door_2 (cast `/Game/Environment/Props/Blueprints/BP_Door` (`self.Door`)))
    (`/Game/Environment/Props/Blueprints/BP_Door.Close` _asbp_door_2)))

(fn `UserConstructionScript`
  (`parent.UserConstructionScript`)
  (bind _returnvalue (`PrimitiveComponent.CreateDynamicMaterialInstance` (`self.Cube`) 0 null))
  (set `self.DynaMat` _returnvalue)
  (bind _outactors (`GameplayStatics.GetAllActorsOfClass` "/Game/Environment/Props/Blueprints/BP_Door.BP_Door_C"))
  (for _array_element _outactors
    (set `self.Door` _array_element)))