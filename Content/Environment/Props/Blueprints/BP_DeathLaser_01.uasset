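; A laser hazard prop that kills the player on touching its box trigger, with an on/off state that other logic can switch.
; Player overlap sends PlayerDieMessage to every ILevel actor and plays an attached Death event inside that loop.
; Activate is a toggle for the particle emitters, point light and box collision; Deactivate calls it only if SwitchOnDeactivate is set.
; BeginPlay toggles the laser off unless DefaultOn is set.
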(event `self.ReceiveBeginPlay`
  (set `self.IsOn` true)
  (if (not (`self.DefaultOn`))
    (`self.Activate`)))

(event `self.Box.OnComponentBeginOverlap`
  (params (OverlappedComponent :type "PrimitiveComponent Object Reference") (OtherActor :type "Actor Object Reference") (OtherComp :type "PrimitiveComponent Object Reference") (OtherBodyIndex :type Integer) (bFromSweep :type Boolean) (SweepResult :type "HitResult Structure (by ref)"))
  ;[1 1 1] Kill Player
  (cast `/Game/Characters/Player/Blueprints/BP_Player_01` OtherActor)
  (bind _outactors (`GameplayStatics.GetAllActorsWithInterface` "/Game/Base/Blueprints/ILevel.ILevel_C"))
  (for _array_element _outactors
    (message `/Game/Base/Blueprints/ILevel.PlayerDie` _array_element)
    (`FMODBlueprintStatics.PlayEventAttached` "/Game/FMOD/Events/Assets/Death.Death" (`self.Box`) "None" (0.0 0.0 0.0) "KeepRelativeOffset")))

(event `/Game/Base/Blueprints/IActivatable.Activate`
  (bind _array (`|MakeArray` (`self.ParticleSystem6`) (`self.ParticleSystem1`) (`self.ParticleSystem2`) (`self.ParticleSystem3`) (`self.ParticleSystem4`) (`self.ParticleSystem5`) (`self.ParticleSystem`)))
  ;[1 1 1] Activate
  (if (`self.IsOn`)
    (for _array_element _array
      (`ParticleSystemComponent.SetEmitterEnable` _array_element "Particle Emitter" false))
    (`LightComponent.SetIntensity` (`self.PointLight`) 0.0)
    (set `self.IsOn` false)
    (`PrimitiveComponent.SetCollisionEnabled` (`self.Box`) "NoCollision")
    (else
      (for _array_element_2 _array
        (`KismetSystemLibrary.PrintString` "Enabling")
        (`ParticleSystemComponent.SetEmitterEnable` _array_element_2 "Particle Emitter" true))
      (`LightComponent.SetIntensity` (`self.PointLight`) (`self.Light Intensity`))
      (set `self.IsOn` true)
      (`PrimitiveComponent.SetCollisionEnabled` (`self.Box`) "QueryOnly"))))

(event `/Game/Base/Blueprints/IActivatable.Deactivate`
  ;[1 1 1] Deactivate
  (if (`self.SwitchOnDeactivate`)
    (`self.Activate`)))

(fn `UserConstructionScript`
  (`LightComponent.SetIntensity` (`self.PointLight`) (`self.Light Intensity`)))