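; Vortex field prop that bends an overlapping laser 90 degrees through a timed goal-direction change, with spinning arrows and swirl particles showing its handedness.
; Activation either toggles the field or cycles it off and back on with reversed visuals, and an optional box enables it while the player is near.
; Enable and Disable switch emitters, ease light and arrow opacity, and delay Active, though the laser turn ignores both Active and Reverse.
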(event `self.ReceiveBeginPlay`
  (set `self.IsOn` true)
  (if (not (`self.DefaultOn`))
    (`self.Disable`)))

(event `self.ReceiveTick`
  (params (DeltaSeconds :type "Float (single-precision)"))
  (bind _arrows (`self.Arrows`))
  (`SceneComponent.K2_SetRelativeRotation` _arrows (`KismetMathLibrary.ComposeRotators` (`SceneComponent.RelativeRotation` _arrows) (`KismetMathLibrary.MakeRotator` 0.0 0.0 (* DeltaSeconds (* (`self.ArrowRotationRate`) (`KismetMathLibrary.SelectFloat` 1.0 -1.0 (`self.Reverse`)))))) false false))

(event `self.LaserBeginOverlap`
  (params (Laser :type "LaserBase Object Reference"))
  ;[1 1 1] Detect Laser
  (`LaserBase.SetGoalDirection` Laser (`KismetMathLibrary.RotateAngleAxis` (`LaserBase.GetVelocity` Laser) -90.0 (0.0 0.0 1.0)) 0.18))

(event `self.LaserTick`
  (params (Laser :type "LaserBase Object Reference") (DeltaSeconds :type "Float (single-precision)"))
  ;[1 1 1] Affect Laser
)

(event `/Game/Base/Blueprints/IActivatable.Activate`
  ;[1 1 1] Activate
  (switch `/Game/Environment/Props/Blueprints/BP_VortexEnum_01` (`self.ActionOnActivate`)
    (:`NewEnumerator0`
      (if (`self.IsOn`)
        (`self.Disable`)
        (`KismetSystemLibrary.Delay` 1.0)
        (`self.Swap`)
        (`self.Enable`)))
    (:`NewEnumerator1`
      (`self.Enable`))))

(event `Swap`
  (bind _arrows (`self.Arrows`))
  ;[1 1 1] Swap
  (set `self.Reverse` (not (`self.Reverse`)))
  (`SceneComponent.SetRelativeScale3D` _arrows (* (`SceneComponent.RelativeScale3D` _arrows) (-1.0 1.0 1.0)))
  (if (`self.Reverse`)
    (`ParticleSystemComponent.SetTemplate` (`self.ParticleSystem`) "/Game/Environment/Props/Particles/PS_VortexLeft_01.PS_VortexLeft_01")
    (else
      (`ParticleSystemComponent.SetTemplate` (`self.ParticleSystem`) "/Game/Environment/Props/Particles/PS_VortexRight_01.PS_VortexRight_01"))))

(event `/Game/Base/Blueprints/IActivatable.Deactivate`
  ;[1 1 1] Deactivate
  (switch `/Game/Environment/Props/Blueprints/BP_VortexEnum_01` (`self.ActionOnActivate`)
    (:`NewEnumerator1`
      (`self.Disable`))))

(event `self.Box1.OnComponentBeginOverlap`
  (params (OverlappedComponent :type "PrimitiveComponent Object Reference") (OtherActor :type "Actor Object Reference") (OtherComp :type "PrimitiveComponent Object Reference") (OtherBodyIndex :type Integer) (bFromSweep :type Boolean) (SweepResult :type "HitResult Structure (by ref)"))
  ;[1 1 1] Detect Player closeby
  (if (not (or (`self.DefaultOn`) (not (`self.UseDetectionBox`))))
    (cast `/Game/Characters/Player/Blueprints/BP_Player_01` OtherActor)
    (`self.Enable`)))

(event `TurnLightOn`
  (bind _returnvalue (`GameplayStatics.GetTimeSeconds`))
  (bind _returnvalue_2 (- _returnvalue (`self.StartTime`)))
  ;[1 1 1] Turn lights on
  (set `self.TurningOn` true)
  (set `self.StartTime` _returnvalue)
  (`/Game/Base/Blueprints/BP_LoopLibrary_01.LoopWithDelay` (and (< _returnvalue_2 1.0) (`self.TurningOn`)) (/ 1.0 20.0)
    (:`Loop Body`
      (`LightComponent.SetIntensity` (`self.PointLight`) (`|EaseFunction` "EaseInOut" _returnvalue_2 0.0 (`self.Light Intensity`)))
      (`MeshComponent.SetScalarParameterValueOnMaterials` (`self.Arrows`) "Opacity" (`|EaseFunction` "EaseInOut" _returnvalue_2 0.0 1.0)))
    (:`Completed`
      (if (`self.TurningOn`)
        (`LightComponent.SetIntensity` (`self.PointLight`) (`self.Light Intensity`))
        (`MeshComponent.SetScalarParameterValueOnMaterials` (`self.Arrows`) "Opacity" 1.0)))))

(event `self.Box1.OnComponentEndOverlap`
  (params (OverlappedComponent :type "PrimitiveComponent Object Reference") (OtherActor :type "Actor Object Reference") (OtherComp :type "PrimitiveComponent Object Reference") (OtherBodyIndex :type Integer))
  ;[1 1 1] Detect player not closeby
  (if (not (or (`self.DefaultOn`) (not (`self.UseDetectionBox`))))
    (cast `/Game/Characters/Player/Blueprints/BP_Player_01` OtherActor)
    (`self.Disable`)))

(event `TurnLightOff`
  (bind _returnvalue (`GameplayStatics.GetTimeSeconds`))
  (bind _returnvalue_2 (- _returnvalue (`self.StartTime`)))
  ;[1 1 1] Turn lights off
  (set `self.TurningOn` false)
  (set `self.StartTime` _returnvalue)
  (`/Game/Base/Blueprints/BP_LoopLibrary_01.LoopWithDelay` (and (< _returnvalue_2 1.0) (not (`self.TurningOn`))) (/ 1.0 20.0)
    (:`Loop Body`
      (`LightComponent.SetIntensity` (`self.PointLight`) (`|EaseFunction` "EaseInOut" _returnvalue_2 (`self.Light Intensity`)))
      (`MeshComponent.SetScalarParameterValueOnMaterials` (`self.Arrows`) "Opacity" (`|EaseFunction` "EaseInOut" _returnvalue_2 1.0)))
    (:`Completed`
      (if (not (`self.TurningOn`))
        (`LightComponent.SetIntensity` (`self.PointLight`) 0.0)
        (`MeshComponent.SetScalarParameterValueOnMaterials` (`self.Arrows`) "Opacity" 0.0)))))

(event `Enable`
  ;[1 1 1] Enable
  (if (not (`self.IsOn`))
    (set `self.IsOn` true)
    (`ParticleSystemComponent.SetEmitterEnable` (`self.ParticleSystem1`) "Particle Emitter" true)
    (`ParticleSystemComponent.SetEmitterEnable` (`self.ParticleSystem`) "Particle Emitter" true)
    (`self.TurnLightOn`)
    (`KismetSystemLibrary.Delay` 1.0)
    (set `self.Active` true)))

(event `Disable`
  ;[1 1 1] Disable
  (if (`self.IsOn`)
    (set `self.IsOn` false)
    (`ParticleSystemComponent.SetEmitterEnable` (`self.ParticleSystem1`) "Particle Emitter" false)
    (`ParticleSystemComponent.SetEmitterEnable` (`self.ParticleSystem`) "Particle Emitter" false)
    (`self.TurnLightOff`)
    (`KismetSystemLibrary.Delay` 1.0)
    (set `self.Active` false)))

(fn `UserConstructionScript`
  (bind _arrows (`self.Arrows`))
  (bind _arrows_2 (`self.Arrows`))
  (bind _detectionsize (`self.DetectionSize`))
  (`parent.UserConstructionScript`)
  (`BoxComponent.SetBoxExtent` (`self.Box1`) (`KismetMathLibrary.MakeVector` _detectionsize _detectionsize 200.0) true)
  (if (`self.Reverse`)
    (`ParticleSystemComponent.SetTemplate` (`self.ParticleSystem`) "/Game/Environment/Props/Particles/PS_VortexLeft_01.PS_VortexLeft_01")
    (`SceneComponent.SetRelativeScale3D` _arrows_2 (`SceneComponent.RelativeScale3D` _arrows_2))
    (else
      (`ParticleSystemComponent.SetTemplate` (`self.ParticleSystem`) "/Game/Environment/Props/Particles/PS_VortexRight_01.PS_VortexRight_01")
      (`SceneComponent.SetRelativeScale3D` _arrows (* (`SceneComponent.RelativeScale3D` _arrows) (`KismetMathLibrary.MakeVector` -1.0 1.0 1.0)))))
  (`LightComponent.SetIntensity` (`self.PointLight`) (`self.Light Intensity`)))