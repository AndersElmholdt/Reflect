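; BP_Receiver_01 is a laser receiver prop that switches linked actors on when a laser hits it.
; It pulls lasers toward its Box; one overlapping the Box is killed, plays a click, turns the light and particles green and calls Activate on the IActivatable actors in Activates.
; A nonzero AutoDisableTime runs a delay-loop countdown on a text render, then turns the light red and deactivates those actors.
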(event `self.ReceiveBeginPlay`
  (`SceneComponent.SetVisibility` (`self.TextRender`) false false))

(event `self.LaserBeginOverlap`
  (params (Laser :type "LaserBase Object Reference"))
  (bind _sm_receiver_01 (`self.SM_Receiver_01`))
  ;[1 1 1] Detect hit
  (if (`PrimitiveComponent.IsOverlappingActor` (`self.Box`) Laser)
    (`LaserBase.Kill` Laser false)
    (`FMODBlueprintStatics.PlayEventAttached` "/Game/FMOD/Events/ButtonClick.ButtonClick" (`self.DefaultSceneRoot`) "None" (0.0 0.0 0.0) "KeepRelativeOffset")
    (`MeshComponent.SetVectorParameterValueOnMaterials` _sm_receiver_01 "LightColor" (0.0 1.0 0.0))
    (`ParticleSystemComponent.SetColorParameter` (`self.ParticleSystem`) "InstanceColorScaleOverLife" (struct :`G` 1.0 :`A` 1.0))
    (for _array_element (`self.Activates`)
      (bind _asiactivatable (cast `/Game/Base/Blueprints/IActivatable` _array_element))
      (`/Game/Base/Blueprints/IActivatable.Activate` _asiactivatable))
    (if (!= (`self.AutoDisableTime`) 0.0)
      (set `self.Timer` 0.0)
      (`SceneComponent.SetVisibility` (`self.TextRender`) true false)
      (`/Game/Base/Blueprints/BP_LoopLibrary_01.LoopWithDelay` (>= (- (`self.AutoDisableTime`) (`self.Timer`)) 0.1) 0.1
        (:`Loop Body`
          (set `self.Timer` (+ (`self.Timer`) 0.1))
          (`TextRenderComponent.K2_SetText` (`self.TextRender`) (`KismetTextLibrary.Conv_DoubleToText` (- (`self.AutoDisableTime`) (`self.Timer`)) "HalfToEven" true 1 324 1 1)))
        (:`Completed`
          (`SceneComponent.SetVisibility` (`self.TextRender`) false false)
          (`MeshComponent.SetVectorParameterValueOnMaterials` _sm_receiver_01 "LightColor" (1.0 0.0 0.0))
          (for _array_element_2 (`self.Activates`)
            (bind _asiactivatable_2 (cast `/Game/Base/Blueprints/IActivatable` _array_element_2))
            (`/Game/Base/Blueprints/IActivatable.Deactivate` _asiactivatable_2)
            (`ParticleSystemComponent.SetColorParameter` (`self.ParticleSystem`) "InstanceColorScaleOverLife" (struct :`R` 1.0 :`A` 1.0))))))))

(event `self.LaserTick`
  (params (Laser :type "LaserBase Object Reference") (DeltaSeconds :type "Float (single-precision)"))
  ;[1 1 1] Suck the laser into the receiver
  (`LaserBase.AddForce` Laser (- (`SceneComponent.K2_GetComponentLocation` (`self.Box`)) (`self.K2_GetActorLocation` Laser)) (* DeltaSeconds (`self.SuctionSpeed`))))

(fn `UserConstructionScript`
  (`parent.UserConstructionScript`))