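; Turbulence field prop that bends lasers passing through it 90 degrees left or right around the vertical axis, depending on Reverse.
; On overlap it stores a single goal velocity from the laser's heading, then while active steers the laser toward it at a capped turn rate.
; Activating it flips the direction, briefly disabling bending and particles before restoring them with the effect mirrored on X.
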(event `self.LaserBeginOverlap`
  (params (Laser :type "LaserBase Object Reference"))
  (bind _returnvalue (`LaserBase.GetVelocity` Laser))
  (if (`self.Reverse`)
    (set `self.GoalVelocity` (`KismetMathLibrary.RotateAngleAxis` _returnvalue -90.0 (0.0 0.0 1.0)))
    (else
      (set `self.GoalVelocity` (`KismetMathLibrary.RotateAngleAxis` _returnvalue 90.0 (0.0 0.0 1.0))))))

(event `self.LaserTick`
  (params (Laser :type "LaserBase Object Reference") (DeltaSeconds :type "Float (single-precision)"))
  (if (`self.Active`)
    (`LaserBase.RotateVelocity` Laser (`self.GoalVelocity`) (* DeltaSeconds 500.0))))

(event `/Game/Base/Blueprints/IActivatable.Activate`
  (bind _particlesystem (`self.ParticleSystem`))
  (set `self.Active` false)
  (set `self.Reverse` (not (`self.Reverse`)))
  (`ParticleSystemComponent.SetEmitterEnable` _particlesystem "Particle Emitter" false)
  (`KismetSystemLibrary.Delay` 2.0)
  (set `self.Active` true)
  (`SceneComponent.SetRelativeScale3D` _particlesystem (* (`SceneComponent.RelativeScale3D` _particlesystem) (`KismetMathLibrary.MakeVector` -1.0 1.0 1.0)))
  (`ParticleSystemComponent.SetEmitterEnable` _particlesystem "Particle Emitter" true))

(fn `UserConstructionScript`
  (`parent.UserConstructionScript`)
  (if (not (`self.Reverse`))
    (`SceneComponent.SetRelativeScale3D` (`self.ParticleSystem`) (-1.0 1.0 1.0))))