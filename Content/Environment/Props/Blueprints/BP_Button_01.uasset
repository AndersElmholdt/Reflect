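; BP_Button_01 is a pressure button that drives linked actors while BP_Player_01 overlaps its Sphere.
; Entering sinks the Main component, then turns it green and calls Activate on the Activates entries through IActivatable.
; Leaving raises it, then turns it red and calls Deactivate.
; Each overlap event stops the opposing MoveComponentTo, so the press and release movements can interrupt each other.
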(event `self.Sphere.OnComponentBeginOverlap`
  (params (OverlappedComponent :type "PrimitiveComponent Object Reference") (OtherActor :type "Actor Object Reference") (OtherComp :type "PrimitiveComponent Object Reference") (OtherBodyIndex :type Integer) (bFromSweep :type Boolean) (SweepResult :type "HitResult Structure (by ref)"))
  (bind _main (`self.Main`))
  (bind _activates (`self.Activates`))
  (bind _main_2 (`self.Main`))
  (cast `/Game/Characters/Player/Blueprints/BP_Player_01` OtherActor)
  (`|ExecutionSequence`
    (:`then_0`
      (goto _label_2 :!via `Stop`))
    (:`then_1`
      (`KismetSystemLibrary.MoveComponentTo` _main_2 (0.0 0.0 -8.0) (struct) false false 0.2 :!label _label)
      (`MeshComponent.SetVectorParameterValueOnMaterials` _main "Color" (0.0 1.0 0.0))
      (for _array_element _activates
        (bind _asiactivatable (cast `/Game/Base/Blueprints/IActivatable` _array_element))
        (`/Game/Base/Blueprints/IActivatable.Activate` _asiactivatable)))))

(event `self.Sphere.OnComponentEndOverlap`
  (params (OverlappedComponent :type "PrimitiveComponent Object Reference") (OtherActor :type "Actor Object Reference") (OtherComp :type "PrimitiveComponent Object Reference") (OtherBodyIndex :type Integer))
  (cast `/Game/Characters/Player/Blueprints/BP_Player_01` OtherActor)
  (`|ExecutionSequence`
    (:`then_0`
      (goto _label :!via `Stop`))
    (:`then_1`
      (`KismetSystemLibrary.MoveComponentTo` (`self.Main`) (0.0 0.0 2.0) (struct) false false 0.2 :!label _label_2)
      (`MeshComponent.SetVectorParameterValueOnMaterials` (`self.Main`) "Color" (1.0 0.0 0.0))
      (for _array_element (`self.Activates`)
        (bind _asiactivatable (cast `/Game/Base/Blueprints/IActivatable` _array_element))
        (`/Game/Base/Blueprints/IActivatable.Deactivate` _asiactivatable)))))

(fn `UserConstructionScript`)