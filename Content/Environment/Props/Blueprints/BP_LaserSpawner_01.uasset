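; BP_LaserSpawner_01 is a rotatable laser emitter prop that fires BP_Laser_01 actors from its Arrow's transform.
; A looping timer started on BeginPlay calls FireLaser every FireRate seconds, spawning only while IsOn, which TurnOn and TurnOff set.
; Activate pauses the timer, eases LocalRotation by a RotationStep yaw, then after a fixed one-second delay fires and restarts the timer.
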(event `self.ReceiveBeginPlay`
  (`KismetSystemLibrary.K2_SetTimer` null "FireLaser" (`self.FireRate`) true))

(event `/Game/Base/Blueprints/IActivatable.Activate`
  (bind _localrotation (`self.LocalRotation`))
  (`KismetSystemLibrary.K2_ClearTimer` null "FireLaser")
  (`KismetSystemLibrary.MoveComponentTo` _localrotation (0.0 0.0 0.0) (`KismetMathLibrary.ComposeRotators` (`SceneComponent.RelativeRotation` _localrotation) (`KismetMathLibrary.MakeRotator` 0.0 0.0 (`self.RotationStep`))) true true (`self.RotationSpeed`))
  (`KismetSystemLibrary.Delay` 1.0)
  (`self.FireLaser`)
  (`KismetSystemLibrary.K2_SetTimer` null "FireLaser" (`self.FireRate`) true))

(event `FireLaser`
  (if (`self.IsOn`)
    (`|SpawnActorFromClass` "/Game/Base/Blueprints/BP_Laser_01.BP_Laser_01_C" (`SceneComponent.K2_GetComponentToWorld` (`self.Arrow`)) "Undefined" "OverrideRootScale")))

(event `TurnOn`
  (set `self.IsOn` true))

(event `TurnOff`
  (set `self.IsOn` false))

(fn `UserConstructionScript`)