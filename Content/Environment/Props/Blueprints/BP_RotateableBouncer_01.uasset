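; Rotatable bouncer prop that redirects lasers, calling Bounce on the laser with the hit normal and an angle clamp.
; Activate eases the mesh by a yaw increment from its current rotation, using a flag to ignore repeat activations mid-turn.
; Deactivate clears that flag and, if ToggleOnDeactivate is set, eases back to the start yaw.
; The construction script applies that start yaw to the mesh.
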(event `self.ReceiveBeginPlay`
  (set `self.IsRotating` false))

(event `/Game/Base/Blueprints/IActivatable.Activate`
  (bind _staticmesh (`self.StaticMesh`))
  (bind (_returnvalue_location _returnvalue_rotation) (`KismetMathLibrary.BreakTransform` (`SceneComponent.GetRelativeTransform` _staticmesh)))
  (if (not (`self.IsRotating`))
    (set `self.IsRotating` true)
    (`KismetSystemLibrary.MoveComponentTo` _staticmesh (0.0 0.0 0.0) (`KismetMathLibrary.ComposeRotators` _returnvalue_rotation (`KismetMathLibrary.MakeRotator` 0.0 0.0 (`self.RotationAngle`))) true true (`self.RotationSpeed`) true)
    (set `self.IsRotating` false)))

(event `/Game/Base/Blueprints/IActivatable.Deactivate`
  (set `self.IsRotating` false)
  (if (`self.ToggleOnDeactivate`)
    (set `self.IsRotating` true)
    (`KismetSystemLibrary.MoveComponentTo` (`self.StaticMesh`) (0.0 0.0 0.0) (`KismetMathLibrary.MakeRotator` 0.0 0.0 (`self.StartRotation`)) true true (`self.RotationSpeed`) true)
    (set `self.IsRotating` false)))

(event `self.LaserHit`
  (params (Laser :type "LaserBase Object Reference") (HitNormal :type "Vector Structure"))
  (`LaserBase.Bounce` Laser HitNormal 1.0 15.0))

(fn `UserConstructionScript`
  (`parent.UserConstructionScript`)
  (`SceneComponent.K2_SetRelativeRotation` (`self.StaticMesh`) (`KismetMathLibrary.MakeRotator` 0.0 0.0 (`self.StartRotation`)) false false))