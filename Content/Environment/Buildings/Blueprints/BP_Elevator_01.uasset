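; BP_Elevator_01 is an elevator building actor whose Glass component swings open and closed and which can serve as the level goal.
; Activate and Deactivate rotate Glass 90 degrees and back with eased MoveComponentTo, playing FMOD audio at the GlobalScope effects volume.
; Box overlaps by BP_Player_01 trigger both when SensorbasedActivation is set.
; If IsGoal is set, the player entering Box1 sends FinishLevelMessage to all ILevel actors.
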(event `/Game/Base/Blueprints/IActivatable.Activate`
  (bind _fmodaudio (`self.FMODAudio`))
  (`FMODAudioComponent.Play` _fmodaudio)
  (bind _asglobal_scope (cast `/Game/GlobalScope` (`GameplayStatics.GetGameInstance`)))
  (`FMODAudioComponent.SetVolume` _fmodaudio (`/Game/GlobalScope.GetEffectsLevel` _asglobal_scope))
  (`KismetSystemLibrary.MoveComponentTo` (`self.Glass`) (0.0 0.0 0.0) (struct :`Yaw` 90.0) true true (`self.AnimationTime`) true))

(event `/Game/Base/Blueprints/IActivatable.Deactivate`
  (bind _fmodaudio1 (`self.FMODAudio1`))
  (`FMODAudioComponent.Play` _fmodaudio1)
  (bind _asglobal_scope (cast `/Game/GlobalScope` (`GameplayStatics.GetGameInstance`)))
  (`FMODAudioComponent.SetVolume` _fmodaudio1 (`/Game/GlobalScope.GetEffectsLevel` _asglobal_scope))
  (`KismetSystemLibrary.MoveComponentTo` (`self.Glass`) (0.0 0.0 0.0) (struct) true true (`self.AnimationTime`) true))

(event `self.Box.OnComponentBeginOverlap`
  (params (OverlappedComponent :type "PrimitiveComponent Object Reference") (OtherActor :type "Actor Object Reference") (OtherComp :type "PrimitiveComponent Object Reference") (OtherBodyIndex :type Integer) (bFromSweep :type Boolean) (SweepResult :type "HitResult Structure (by ref)"))
  (cast `/Game/Characters/Player/Blueprints/BP_Player_01` OtherActor)
  (if (`self.SensorbasedActivation`)
    (`self.Activate`)))

(event `self.Box.OnComponentEndOverlap`
  (params (OverlappedComponent :type "PrimitiveComponent Object Reference") (OtherActor :type "Actor Object Reference") (OtherComp :type "PrimitiveComponent Object Reference") (OtherBodyIndex :type Integer))
  (cast `/Game/Characters/Player/Blueprints/BP_Player_01` OtherActor)
  (if (`self.SensorbasedActivation`)
    (`self.Deactivate`)))

(event `self.Box1.OnComponentBeginOverlap`
  (params (OverlappedComponent :type "PrimitiveComponent Object Reference") (OtherActor :type "Actor Object Reference") (OtherComp :type "PrimitiveComponent Object Reference") (OtherBodyIndex :type Integer) (bFromSweep :type Boolean) (SweepResult :type "HitResult Structure (by ref)"))
  (cast `/Game/Characters/Player/Blueprints/BP_Player_01` OtherActor)
  (if (`self.IsGoal`)
    (bind _outactors (`GameplayStatics.GetAllActorsWithInterface` "/Game/Base/Blueprints/ILevel.ILevel_C"))
    (for _array_element _outactors
      (message `/Game/Base/Blueprints/ILevel.FinishLevel` _array_element))))

(fn `UserConstructionScript`)