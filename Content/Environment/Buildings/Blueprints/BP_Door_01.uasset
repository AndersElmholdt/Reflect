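; Sliding double door that opens on Activate and closes on Deactivate, with attached sound events and a red/green light set through a material parameter.
; A front unlocker rotates via MoveComponentTo, while AnimateDoors eases both panels from their current positions to open or closed offsets.
; The slide is time-based in a fixed-delay loop rather than Tick or Timeline; the custom WhileLoopWithDelay macro's call is disconnected in favor of LoopWithDelay.
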(event `/Game/Base/Blueprints/IActivatable.Deactivate`
  (bind _defaultsceneroot (`self.DefaultSceneRoot`))
  (bind _doorunlockerfront (`self.DoorUnlockerFront`))
  (bind _returnvalue_location (`KismetMathLibrary.BreakTransform` (`SceneComponent.GetRelativeTransform` _doorunlockerfront)))
  (bind _returnvalue_location_2 (`KismetMathLibrary.BreakTransform` (`SceneComponent.GetRelativeTransform` (`self.DoorLeft`))))
  (bind _returnvalue_location_3 (`KismetMathLibrary.BreakTransform` (`SceneComponent.GetRelativeTransform` (`self.DoorRight`))))
  ;[1 1 1] Deactivate the Door
  (set `self.LeftStartPos` _returnvalue_location_2)
  (set `self.RightStartPos` _returnvalue_location_3)
  (set `self.LeftTargetPos` (0.0 0.0 0.0))
  (set `self.RightTargetPos` (0.0 0.0 0.0))
  (set `self.StartSeconds` (`GameplayStatics.GetTimeSeconds`))
  (`self.AnimateDoors`)
  (`FMODBlueprintStatics.PlayEventAttached` "/Game/FMOD/Events/Assets/Door/DoorDoorClose.DoorDoorClose" _defaultsceneroot "None" (0.0 0.0 0.0) "KeepRelativeOffset")
  (`KismetSystemLibrary.Delay` (`self.DoorAnimationTime`))
  (`FMODBlueprintStatics.PlayEventAttached` "/Game/FMOD/Events/Assets/Door/DoorClickClose.DoorClickClose" _defaultsceneroot "None" (0.0 0.0 0.0) "KeepRelativeOffset")
  (`KismetSystemLibrary.MoveComponentTo` _doorunlockerfront _returnvalue_location (struct) true true (`self.DoorUnlockTime`) true)
  (`MeshComponent.SetVectorParameterValueOnMaterials` (`self.Extra`) "LightColor" (1.0 0.0 0.0)))

(event `/Game/Base/Blueprints/IActivatable.Activate`
  (bind _doorunlockerfront (`self.DoorUnlockerFront`))
  (bind _defaultsceneroot (`self.DefaultSceneRoot`))
  (bind _returnvalue_location (`KismetMathLibrary.BreakTransform` (`SceneComponent.GetRelativeTransform` _doorunlockerfront)))
  (bind _returnvalue_location_2 (`KismetMathLibrary.BreakTransform` (`SceneComponent.GetRelativeTransform` (`self.DoorLeft`))))
  (bind _returnvalue_location_3 (`KismetMathLibrary.BreakTransform` (`SceneComponent.GetRelativeTransform` (`self.DoorRight`))))
  ;[1 1 1] Activate the Door
  (`FMODBlueprintStatics.PlayEventAttached` "/Game/FMOD/Events/Assets/Door/DoorSteam.DoorSteam" _defaultsceneroot "None" (0.0 0.0 0.0) "KeepRelativeOffset")
  (`KismetSystemLibrary.MoveComponentTo` _doorunlockerfront _returnvalue_location (struct :`Pitch` 170.0) true true (`self.DoorUnlockTime`) true)
  ;[1 1 1] Deactivate the Door
  (`FMODBlueprintStatics.PlayEventAttached` "/Game/FMOD/Events/Assets/Door/DoorDoorOpen.DoorDoorOpen" _defaultsceneroot "None" (0.0 0.0 0.0) "KeepRelativeOffset")
  (`FMODBlueprintStatics.PlayEventAttached` "/Game/FMOD/Events/Assets/Door/DoorClickOpen.DoorClickOpen" _defaultsceneroot "None" (0.0 0.0 0.0) "KeepRelativeOffset")
  (`MeshComponent.SetVectorParameterValueOnMaterials` (`self.Extra`) "LightColor" (0.0 1.0 0.0))
  (set `self.LeftStartPos` _returnvalue_location_2)
  (set `self.RightStartPos` _returnvalue_location_3)
  (set `self.LeftTargetPos` (-165.0 0.0 0.0))
  (set `self.RightTargetPos` (165.0 0.0 0.0))
  (set `self.StartSeconds` (`GameplayStatics.GetTimeSeconds`))
  (`self.AnimateDoors`))

(event `AnimateDoors`
  (bind _returnvalue (/ (- (`GameplayStatics.GetTimeSeconds`) (`self.StartSeconds`)) (`self.DoorAnimationTime`)))
  ;[1 1 1] Animate Doors
  (`/Game/Base/Blueprints/BP_LoopLibrary_01.LoopWithDelay` (<= _returnvalue 1.0) (/ 1.0 144.0)
    (:`Loop Body`
      (`SceneComponent.K2_SetRelativeLocation` (`self.DoorLeft`) (`|EaseFunction` "EaseInOut" _returnvalue (`self.LeftStartPos`) (`self.LeftTargetPos`)) false false)
      (`SceneComponent.K2_SetRelativeLocation` (`self.DoorRight`) (`|EaseFunction` "EaseInOut" _returnvalue (`self.RightStartPos`) (`self.RightTargetPos`)) false false))))

(fn `UserConstructionScript`)