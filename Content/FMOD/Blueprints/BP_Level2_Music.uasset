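; BP_Level2_Music is an FMOD music actor, named for Level 2, that keeps its audio volume in line with the game's music level setting.
; Both the construction script and an UpdateVolume event cast the game instance to GlobalScope and apply its music level to the FMODAudio component.
; Nothing in the file calls UpdateVolume, and the default BeginPlay, overlap and Tick events are unused.
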(event `/Game/FMOD/Blueprints/ISoundPlayers.UpdateVolume`
  (bind _asglobal_scope (cast `/Game/GlobalScope` (`GameplayStatics.GetGameInstance`)))
  (`FMODAudioComponent.SetVolume` (`self.FMODAudio`) (`/Game/GlobalScope.GetMusicLevel` _asglobal_scope)))

(fn `UserConstructionScript`
  (bind _asglobal_scope (cast `/Game/GlobalScope` (`GameplayStatics.GetGameInstance`)))
  (`FMODAudioComponent.SetVolume` (`self.FMODAudio`) (`/Game/GlobalScope.GetMusicLevel` _asglobal_scope)))