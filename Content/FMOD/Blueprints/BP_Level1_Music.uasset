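; BP_Level1_Music is a Blueprint that controls the volume of the Level 1 music.
; Both the construction script and an UpdateVolume event set the Level1Music volume from the music level stored in the GlobalScope game instance.
; If the game instance is not a GlobalScope, the volume is left unchanged.
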(event `/Game/FMOD/Blueprints/ISoundPlayers.UpdateVolume`
  (bind _asglobal_scope (cast `/Game/GlobalScope` (`GameplayStatics.GetGameInstance`)))
  (`FMODAudioComponent.SetVolume` (`self.Level1Music`) (`/Game/GlobalScope.GetMusicLevel` _asglobal_scope)))

(fn `UserConstructionScript`
  (bind _asglobal_scope (cast `/Game/GlobalScope` (`GameplayStatics.GetGameInstance`)))
  (`FMODAudioComponent.SetVolume` (`self.Level1Music`) (`/Game/GlobalScope.GetMusicLevel` _asglobal_scope)))