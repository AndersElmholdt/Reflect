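; Player character for a laser shooter that spawns an attached gun and tutorial HUD, and reports laser-hit deaths to ILevel actors.
; Tick hot-swaps gamepad and mouse aiming, moves relative to a step-rotated spring-arm camera, and toggles a looping footstep timer.
; Held fire spawns lasers through a rate-limited DoOnce and notifies ILevel actors.
; An aim trace draws debug lines colored by whether the target is a LaserBouncer.
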(event `self.ReceiveBeginPlay`
  (bind _mesh (`self.Mesh`))
  (set `self.IsAlive` true)
  (bind _returnvalue (`|SpawnActorFromClass` "/Game/Characters/Player/Blueprints/BP_Gun_01.BP_Gun_01_C" (`SceneComponent.K2_GetComponentToWorld` _mesh) "AlwaysSpawn" "OverrideRootScale"))
  (bind _output_get (set `self.Gun` _returnvalue))
  (`self.K2_AttachToComponent` _output_get _mesh "GunSocket" "SnapToTarget" "SnapToTarget" "SnapToTarget" true)
  (bind _asbp_gun_01 (cast `/Game/Characters/Player/Blueprints/BP_Gun_01` (`self.Gun`)))
  (set `self.GunArrow` (`/Game/Characters/Player/Blueprints/BP_Gun_01.Arrow` _asbp_gun_01))
  (if (not (`KismetSystemLibrary.IsValid` (`self.Hud Reference`)))
    (bind _returnvalue_2 (`|CreateWidget` "/Game/HUD/Tutorial/Blueprints/BP_TutorialHUD_01.BP_TutorialHUD_01_C"))
    (bind _output_get_2 (set `self.Hud Reference` _returnvalue_2))
    (`UserWidget.AddToViewport` _output_get_2 0)))

(event `InputAction|Shoot`
  (params (Key :type "Key Structure" :default "AnyKey"))
  ;[1 1 1] Shooting
  (:`Pressed`
    (set `self.IsShooting` true))
  (:`Released`
    (set `self.IsShooting` false)))

(event `ResetFire`
  (bind (_returnvalue_location _returnvalue_rotation _returnvalue_scale) (`KismetMathLibrary.BreakTransform` (`self.GetTransform`)))
  ;[1 1 1] Shooting
  (goto _label :!via `Reset`))

(event `self.ReceiveTick`
  (params (DeltaSeconds :type "Float (single-precision)"))
  (bind _returnvalue (`self.K2_GetActorLocation`))
  (bind (_returnvalue_location _returnvalue_rotation _returnvalue_scale) (`KismetMathLibrary.BreakTransform` (`self.GetTransform`)))
  (bind (_returnvalue_x _returnvalue_y _returnvalue_z) (`KismetMathLibrary.BreakVector` (`self.K2_GetActorLocation`)))
  (bind _returnvalue_2 (`SceneComponent.K2_GetComponentLocation` (`self.GunArrow`)))
  (bind (_worldlocation _worlddirection) (`PlayerController.DeprojectMousePositionToWorld` (`GameplayStatics.GetPlayerController` 0)))
  (bind _returnvalue_3 (`KismetMathLibrary.MakeVector` (`self.GetInputAxisValue`) (`self.GetInputAxisValue`)))
  (bind _returnvalue_4 (* (`KismetMathLibrary.RotateAngleAxis` (`KismetMathLibrary.ClampVectorSize` (`KismetMathLibrary.MakeVector` (`self.GetInputAxisValue`) (`self.GetInputAxisValue`)) 0.0 1.0) (`self.CameraAngle`) (0.0 0.0 1.0)) (* DeltaSeconds (`self.MoveSpeed`))))
  ;[1 1 1] Translate Character
  (if (`self.IsAlive`)
    (`|ExecutionSequence`
      (:`then_0`
        ;[1 1 1] Hotswap Gamepad/Mouse
        (if (!= (+ (`KismetMathLibrary.Abs` (`self.GetInputAxisKeyValue`)) (`KismetMathLibrary.Abs` (`self.GetInputAxisKeyValue`)) (`KismetMathLibrary.Abs` (`self.GetInputAxisKeyValue`)) (`KismetMathLibrary.Abs` (`self.GetInputAxisKeyValue`))) 0.0)
          (set `self.GamepadControl` true)
          (elif (!= (`self.GetInputAxisKeyValue`) 0.0)
            (set `self.GamepadControl` false))))
      (:`then_1`
        ;[1 1 1] Shooting
        (if (`self.IsShooting`)
          (`/Engine/EditorBlueprintResources/StandardMacros.DoOnce` false :!label _label
            (:`Completed`
              (`|SpawnActorFromClass` "/Game/Base/Blueprints/BP_Laser_01.BP_Laser_01_C" (`KismetMathLibrary.MakeTransform` (+ (`SceneComponent.K2_GetComponentLocation` (`self.GunArrow`)) (* (`self.GetActorForwardVector`) (`self.LaserSpawnOffset`))) _returnvalue_rotation _returnvalue_scale) "Undefined" "OverrideRootScale")
              (bind _outactors (`GameplayStatics.GetAllActorsWithInterface` "/Game/Base/Blueprints/ILevel.ILevel_C"))
              (for _array_element _outactors
                (message `/Game/Base/Blueprints/ILevel.DetectLaser` _array_element))
              (`KismetSystemLibrary.Delay` (/ 1.0 (`self.FireRate`)))
              (`self.ResetFire`)))))
      (:`then_2`
        (`self.AddMovementInput` _returnvalue_4 0.4)
        ;[1 1 1] Rotate Character
        (if (`self.GamepadControl`)
          ;;[1 1 1] Controller Rotation
          (if (> (`KismetMathLibrary.VSizeSquared` _returnvalue_3) 0.25)
            (`Controller.SetControlRotation` (`self.GetController`) (`KismetMathLibrary.MakeRotFromX` (`KismetMathLibrary.RotateAngleAxis` _returnvalue_3 (`self.CameraAngle`) (0.0 0.0 1.0))))
            ;[1 1 1] Aim Line Trace
            (bind _outactors_2 (`GameplayStatics.GetAllActorsOfClass` "/Game/Base/Blueprints/BP_Laser_01.BP_Laser_01_C" :!label _label_2))
            (bind (_outhit _returnvalue_5) (`KismetSystemLibrary.LineTraceSingle` _returnvalue (+ _returnvalue (* (`KismetMathLibrary.GetForwardVector` (`Controller.GetControlRotation` (`self.GetController`))) (`self.AimTraceLength`))) "TraceTypeQuery1" false _outactors_2))
            (if _returnvalue_5
              (if (`KismetSystemLibrary.DoesImplementInterface` (`.HitActor` (`GameplayStatics.BreakHitResult` _outhit)) "/Script/Reflect.LaserBouncer")
                (`KismetSystemLibrary.DrawDebugLine` _returnvalue_2 (`.Location` (`GameplayStatics.BreakHitResult` _outhit)) (struct :`G` 0.473697 :`B` 1.0 :`A` 1.0) 0.0 10.0)
                (else
                  (`KismetSystemLibrary.DrawDebugLine` _returnvalue_2 (`.Location` (`GameplayStatics.BreakHitResult` _outhit)) (struct :`R` 1.0 :`A` 1.0) 0.0 10.0)))))
          (else
            ;;[1 1 1] Mouse Rotation
            (`Controller.SetControlRotation` (`self.GetController`) (`KismetMathLibrary.MakeRotFromX` (`KismetMathLibrary.Normal` (- (- _worldlocation (* _worlddirection (/ (- (.z _worldlocation) _returnvalue_z) (.z _worlddirection)))) (`self.K2_GetActorLocation`)))))
            (goto _label_2))))
      (:`then_3`
        (if (> (`KismetMathLibrary.VSizeSquared` _returnvalue_4) 0.2)
          (`/Engine/EditorBlueprintResources/StandardMacros.DoOnce` false :!label _label_3
            (:`Completed`
              (`KismetSystemLibrary.K2_SetTimer` null "PlayFootstep" 0.5 true)))
          (else
            (`KismetSystemLibrary.K2_ClearTimer` null "PlayFootstep")
            (goto _label_3 :!via `Reset`)))))
    (else
      (`KismetSystemLibrary.K2_ClearTimer` null "PlayFootstep"))))

(event `PlayFootstep`
  (`FMODBlueprintStatics.PlayEventAttached` "/Game/FMOD/Events/Assets/Character/Footsteps.Footsteps" (`self.Mesh`) "None" (0.0 0.0 0.0) "KeepRelativeOffset"))

(event `SetZoom`
  (params (NewZoom :type "Float (double-precision)" :default 0.0) (InterpolationTime :type "Float (double-precision)" :default 1.0))
  (bind _zoomgoal (`self.ZoomGoal`))
  (bind _targetarmlength (`SpringArmComponent.TargetArmLength` (`self.SpringArm`)))
  ;[1 1 1] Set Zoom
  (if (== InterpolationTime 0.0)
    (set `SpringArmComponent.TargetArmLength` 0.0 (`self.SpringArm`))
    (else
      (if (== NewZoom 0.0)
        (set `self.ZoomGoal` (`self.DefaultZoom`))
        (else
          (set `self.ZoomGoal` NewZoom)))
      (set `self.StartSeconds` (`GameplayStatics.GetTimeSeconds`))
      (`/Game/Base/Blueprints/BP_LoopLibrary_01.LoopWithDelay` (!= _zoomgoal _targetarmlength) (/ 1.0 144.0)
        (:`Loop Body`
          (set `SpringArmComponent.TargetArmLength` (`|EaseFunction` "EaseInOut" (`KismetMathLibrary.FClamp` (/ (- (`GameplayStatics.GetTimeSeconds`) (`self.StartSeconds`)) InterpolationTime)) _targetarmlength _zoomgoal) (`self.SpringArm`)))))))

(event `InputAxis|ZoomOut`
  (params (AxisValue :type "Float (single-precision)"))
  ;[1 1 1] Zoom Camera (DEPRECATED)
)

(event `InputAction|RotateCameraRight`
  (params (Key :type "Key Structure" :default "AnyKey"))
  (bind _springarm (`self.SpringArm`))
  (bind _returnvalue (`SceneComponent.GetRelativeTransform` _springarm))
  ;[1 1 1] Rotate Camera
  (:`Pressed`
    (set `self.CameraAngle` (mod (+ (`self.CameraAngle`) (* (`self.CameraRotationStep`) -1.0)) 360.0))
    (`KismetSystemLibrary.MoveComponentTo` _springarm (0.0 0.0 0.0) (`KismetMathLibrary.MakeRotator` (.roll (.rotation _returnvalue)) (.pitch (.rotation _returnvalue)) (`self.CameraAngle`)) true true 0.5 true :!label _label_4)))

(event `self.LaserHit`
  (params (Laser :type "LaserBase Object Reference") (HitNormal :type "Vector Structure"))
  ;[1 1 1] Detect Laser Hit
  (bind _outactors (`GameplayStatics.GetAllActorsWithInterface` "/Game/Base/Blueprints/ILevel.ILevel_C"))
  (for _array_element _outactors
    (bind _asilevel (cast `/Game/Base/Blueprints/ILevel` _array_element))
    (`/Game/Base/Blueprints/ILevel.PlayerDie` _asilevel)
    (`FMODBlueprintStatics.PlayEventAttached` "/Game/FMOD/Events/Assets/Death.Death" (`self.CapsuleComponent`) "None" (0.0 0.0 0.0) "KeepRelativeOffset"))
  (`LaserBase.Kill` Laser true))

(event `InputAction|RotateCameraLeft`
  (params (Key :type "Key Structure" :default "AnyKey"))
  ;[1 1 1] Rotate Camera
  (:`Pressed`
    (set `self.CameraAngle` (mod (+ (`self.CameraAngle`) (`self.CameraRotationStep`)) 360.0))
    (goto _label_4)))

(fn `UserConstructionScript`)