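; BP_ArrowDecalGroup_01 is an actor that manages a group of arrow decals and switches their color between normal and activated states.
; The construction script creates shared dynamic material instances for Multi, Single and Turn arrows, tints them with DecalColor, and assigns one to each Decals entry by its ArrowType.
; Activate and Deactivate set the Color parameter on those shared instances to ActivationColor or DecalColor, recoloring the whole group at once.
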(event `/Game/Base/Blueprints/IActivatable.Activate`
  (`MaterialInstanceDynamic.SetVectorParameterValue` (`self.DynaMatMulti`) "Color" (`self.ActivationColor`))
  (`MaterialInstanceDynamic.SetVectorParameterValue` (`self.DynaMatSingle`) "Color" (`self.ActivationColor`))
  (`MaterialInstanceDynamic.SetVectorParameterValue` (`self.DynaMatTurn`) "Color" (`self.ActivationColor`)))

(event `/Game/Base/Blueprints/IActivatable.Deactivate`
  (`MaterialInstanceDynamic.SetVectorParameterValue` (`self.DynaMatMulti`) "Color" (`self.DecalColor`))
  (`MaterialInstanceDynamic.SetVectorParameterValue` (`self.DynaMatSingle`) "Color" (`self.DecalColor`))
  (`MaterialInstanceDynamic.SetVectorParameterValue` (`self.DynaMatTurn`) "Color" (`self.DecalColor`)))

(fn `UserConstructionScript`
  (`|ExecutionSequence`
    (:`then_0`
      (bind _returnvalue (`KismetMaterialLibrary.CreateDynamicMaterialInstance` "/Game/DeferedDecals/Materials/M_Decal_Arrow_Multi.M_Decal_Arrow_Multi"))
      (bind _output_get (set `self.DynaMatMulti` _returnvalue))
      (`MaterialInstanceDynamic.SetVectorParameterValue` _output_get "Color" (`self.DecalColor`)))
    (:`then_1`
      (bind _returnvalue_2 (`KismetMaterialLibrary.CreateDynamicMaterialInstance` "/Game/DeferedDecals/Materials/M_Decal_Arrow_Single.M_Decal_Arrow_Single"))
      (bind _output_get_2 (set `self.DynaMatSingle` _returnvalue_2))
      (`MaterialInstanceDynamic.SetVectorParameterValue` _output_get_2 "Color" (`self.DecalColor`)))
    (:`then_2`
      (bind _returnvalue_3 (`KismetMaterialLibrary.CreateDynamicMaterialInstance` "/Game/DeferedDecals/Materials/M_Decal_Arrow_Turn.M_Decal_Arrow_Turn"))
      (bind _output_get_3 (set `self.DynaMatTurn` _returnvalue_3))
      (`MaterialInstanceDynamic.SetVectorParameterValue` _output_get_3 "Color" (`self.DecalColor`)))
    (:`then_3`
      (for _array_element (`self.Decals`)
        (switch `/Game/DeferedDecals/Blueprints/BP_ArrowType_01` (`/Game/DeferedDecals/Blueprints/BP_ArrowDecal_01.ArrowType` _array_element)
          (:`NewEnumerator0`
            (bind _decal (`DecalActor.Decal` _array_element))
            (`DecalComponent.SetDecalMaterial` _decal (`self.DynaMatMulti`)))
          (:`NewEnumerator1`
            (`DecalComponent.SetDecalMaterial` _decal (`self.DynaMatSingle`)))
          (:`NewEnumerator2`
            (`DecalComponent.SetDecalMaterial` _decal (`self.DynaMatTurn`))))))))