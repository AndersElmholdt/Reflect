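; BP_Laser_01 is a laser actor, apparently a fired shot, that carries a LaserShootSound audio component.
; Its logic only sets that sound's volume from the GlobalScope game instance.
; The construction script applies the music level, then BeginPlay overrides it with the effects level.
; Movement, collision and damage have no logic in these graphs.
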(event `self.ReceiveBeginPlay`
  (bind _asglobal_scope (cast `/Game/GlobalScope` (`GameplayStatics.GetGameInstance`)))
  (`FMODAudioComponent.SetVolume` (`self.LaserShootSound`) (`/Game/GlobalScope.GetEffectsLevel` _asglobal_scope)))

(event `self.ReceiveTick`
  (params (DeltaSeconds :type "Float (single-precision)")))

(fn `UserConstructionScript`
  (bind _asglobal_scope (cast `/Game/GlobalScope` (`GameplayStatics.GetGameInstance`)))
  (`FMODAudioComponent.SetVolume` (`self.LaserShootSound`) (`/Game/GlobalScope.GetMusicLevel` _asglobal_scope)))