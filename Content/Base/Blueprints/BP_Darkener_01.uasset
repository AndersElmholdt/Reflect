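; A darkened volume that fades to transparent while the player is inside it and back to near-opaque when they leave.
; Overlap events on the Box, filtered to BP_Player_01, run a delayed loop lerping the Cube material's Opacity over TransitionTime.
; The Activating flag cancels the opposite fade, which resumes from the current opacity.
; The construction script sizes Box and Cube from Size and offsets the trigger by OverlapTransformOffset.
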(event `self.Box.OnComponentBeginOverlap`
  (params (OverlappedComponent :type "PrimitiveComponent Object Reference") (OtherActor :type "Actor Object Reference") (OtherComp :type "PrimitiveComponent Object Reference") (OtherBodyIndex :type Integer) (bFromSweep :type Boolean) (SweepResult :type "HitResult Structure (by ref)"))
  (bind _returnvalue (`KismetMathLibrary.Lerp` (`self.StartOpacity`) 0.0 (`KismetMathLibrary.FClamp` (/ (- (`GameplayStatics.GetTimeSeconds`) (`self.StartTime`)) (`self.TransitionTime`)))))
  (cast `/Game/Characters/Player/Blueprints/BP_Player_01` OtherActor)
  (set `self.Activating` true)
  (set `self.StartOpacity` (`self.Opacity`))
  (set `self.StartTime` (`GameplayStatics.GetTimeSeconds`))
  (`/Game/Base/Blueprints/BP_LoopLibrary_01.LoopWithDelay` (and (< (- (`GameplayStatics.GetTimeSeconds`) (`self.StartTime`)) (`self.TransitionTime`)) (`self.Activating`)) (/ 1.0 144.0)
    (:`Loop Body`
      (`MeshComponent.SetScalarParameterValueOnMaterials` (`self.Cube`) "Opacity" _returnvalue)
      (set `self.Opacity` _returnvalue))))

(event `self.Box.OnComponentEndOverlap`
  (params (OverlappedComponent :type "PrimitiveComponent Object Reference") (OtherActor :type "Actor Object Reference") (OtherComp :type "PrimitiveComponent Object Reference") (OtherBodyIndex :type Integer))
  (bind _returnvalue (`KismetMathLibrary.Lerp` (`self.StartOpacity`) 0.9 (`KismetMathLibrary.FClamp` (/ (- (`GameplayStatics.GetTimeSeconds`) (`self.StartTime`)) (`self.TransitionTime`)))))
  (cast `/Game/Characters/Player/Blueprints/BP_Player_01` OtherActor)
  (set `self.Activating` false)
  (set `self.StartOpacity` (`self.Opacity`))
  (set `self.StartTime` (`GameplayStatics.GetTimeSeconds`))
  (`/Game/Base/Blueprints/BP_LoopLibrary_01.LoopWithDelay` (and (< (- (`GameplayStatics.GetTimeSeconds`) (`self.StartTime`)) (`self.TransitionTime`)) (not (`self.Activating`))) (/ 1.0 144.0)
    (:`Loop Body`
      (`MeshComponent.SetScalarParameterValueOnMaterials` (`self.Cube`) "Opacity" _returnvalue)
      (set `self.Opacity` _returnvalue))))

(fn `UserConstructionScript`
  (bind _size (`self.Size`))
  (bind _box (`self.Box`))
  (`BoxComponent.SetBoxExtent` _box _size true)
  (`SceneComponent.K2_SetRelativeTransform` _box (`self.OverlapTransformOffset`) false false)
  (`SceneComponent.SetRelativeScale3D` (`self.Cube`) (/ _size 50.0)))