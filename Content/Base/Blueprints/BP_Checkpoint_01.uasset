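; BP_Checkpoint_01 is a checkpoint trigger that updates the spawn point when BP_Player_01 overlaps its box.
; The overlap calls Activate, which finds every actor implementing ILevel and sends it SetSpawnPointMessage with the checkpoint's X and Y at a fixed Z, plus a debug print.
; The construction script sizes the box from the Size variable.
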(event `self.Box.OnComponentBeginOverlap`
  (params (OverlappedComponent :type "PrimitiveComponent Object Reference") (OtherActor :type "Actor Object Reference") (OtherComp :type "PrimitiveComponent Object Reference") (OtherBodyIndex :type Integer) (bFromSweep :type Boolean) (SweepResult :type "HitResult Structure (by ref)"))
  (cast `/Game/Characters/Player/Blueprints/BP_Player_01` OtherActor)
  (`self.Activate`))

(event `/Game/Base/Blueprints/IActivatable.Activate`
  (bind (_returnvalue_x _returnvalue_y) (`KismetMathLibrary.BreakVector` (`self.K2_GetActorLocation`)))
  (bind _outactors (`GameplayStatics.GetAllActorsWithInterface` "/Game/Base/Blueprints/ILevel.ILevel_C"))
  (for _array_element _outactors
    (message `/Game/Base/Blueprints/ILevel.SetSpawnPoint` _array_element (`KismetMathLibrary.MakeVector` _returnvalue_x _returnvalue_y 100.0))
    (`KismetSystemLibrary.PrintString` "Hello")))

(fn `UserConstructionScript`
  (`BoxComponent.SetBoxExtent` (`self.Box`) (`self.Size`) true))