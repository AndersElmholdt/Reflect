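; HUD Blueprint that draws a custom mouse cursor reticle while the player is not using gamepad control.
; Each DrawHUD reads the GamepadControl flag on the BP_Player_01 pawn and, when it is off, draws M_Reticle centered on the mouse position.
; The position is shifted by half the difference between HUD canvas and viewport sizes to keep the reticle aligned when they differ.
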(event `self.ReceiveDrawHUD`
  (params (SizeX :type Integer) (SizeY :type Integer))
  (bind _returnvalue (/ 32.0 2.0))
  (bind (_locationx _locationy) (`PlayerController.GetMousePosition` (`GameplayStatics.GetPlayerController` 0)))
  (bind (_sizex _sizey) (`PlayerController.GetViewportSize` (`GameplayStatics.GetPlayerController` 0)))
  ;[1 1 1] Draw Cursor
  (bind _asbp_player_01 (cast `/Game/Characters/Player/Blueprints/BP_Player_01` (`GameplayStatics.GetPlayerPawn` 0)))
  (if (not (`/Game/Characters/Player/Blueprints/BP_Player_01.GamepadControl` _asbp_player_01))
    (`self.DrawMaterial` "/Game/DeferedDecals/Materials/M_Reticle.M_Reticle" (- (+ _locationx (/ (`KismetMathLibrary.Conv_IntToDouble` (- SizeX _sizex)) 2.0)) _returnvalue) (- (+ _locationy (/ (`KismetMathLibrary.Conv_IntToDouble` (- SizeY _sizey)) 2.0)) _returnvalue) 32.0 32.0 0.0 0.0 1.0 1.0)))

(fn `UserConstructionScript`)