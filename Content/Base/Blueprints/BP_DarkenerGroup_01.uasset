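; BP_DarkenerGroup_01 controls a group of darkener walls, fading them clear on Activate and nearly opaque on Deactivate.
; Both events record the start time and opacity and use a time-based Lerp over TransitionTime to set the Opacity material parameter on each wall's static meshes.
; A high-rate LoopWithDelay timing loop checks the Activating flag so an opposite call ends it, though its body appears empty here.
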(event `/Game/Base/Blueprints/IActivatable.Activate`
  (bind _returnvalue (`KismetMathLibrary.Lerp` (`self.StartOpacity`) 0.0 (`KismetMathLibrary.FClamp` (/ (- (`GameplayStatics.GetTimeSeconds`) (`self.StartTime`)) (`self.TransitionTime`)))))
  (set `self.Activating` true)
  (set `self.StartOpacity` (`self.Opacity`))
  (set `self.StartTime` (`GameplayStatics.GetTimeSeconds`))
  (`/Game/Base/Blueprints/BP_LoopLibrary_01.LoopWithDelay` (and (< (- (`GameplayStatics.GetTimeSeconds`) (`self.StartTime`)) (`self.TransitionTime`)) (`self.Activating`)) (/ 1.0 144.0)
    (:`Loop Body`
      _)
    (:`Completed`
      _))
  (for _array_element (`self.DarkenerWalls`)
    (for _array_element_2 (`self.K2_GetComponentsByClass` _array_element "/Script/Engine.StaticMeshComponent")
      (`MeshComponent.SetScalarParameterValueOnMaterials` _array_element_2 "Opacity" _returnvalue)
      (set `self.Opacity` _returnvalue))))

(event `/Game/Base/Blueprints/IActivatable.Deactivate`
  (bind _returnvalue (`KismetMathLibrary.Lerp` (`self.StartOpacity`) 0.9 (`KismetMathLibrary.FClamp` (/ (- (`GameplayStatics.GetTimeSeconds`) (`self.StartTime`)) (`self.TransitionTime`)))))
  (set `self.Activating` false)
  (set `self.StartOpacity` (`self.Opacity`))
  (set `self.StartTime` (`GameplayStatics.GetTimeSeconds`))
  (`/Game/Base/Blueprints/BP_LoopLibrary_01.LoopWithDelay` (and (< (- (`GameplayStatics.GetTimeSeconds`) (`self.StartTime`)) (`self.TransitionTime`)) (not (`self.Activating`))) (/ 1.0 144.0)
    (:`Loop Body`
      _)
    (:`Completed`
      _))
  (for _array_element (`self.DarkenerWalls`)
    (for _array_element_2 (`self.K2_GetComponentsByClass` _array_element "/Script/Engine.StaticMeshComponent")
      (`MeshComponent.SetScalarParameterValueOnMaterials` _array_element_2 "Opacity" _returnvalue)
      (set `self.Opacity` _returnvalue))))

(fn `UserConstructionScript`)